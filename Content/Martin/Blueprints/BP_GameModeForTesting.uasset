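; Test game mode that handles player spawning, checkpoint respawns and puzzle resets.
; On login it stores the controller and a PlayerStart transform, then restarts the player and binds Respawn to the pawn's destruction.
; Respawn restarts that player at the stored transform and calls CallResetPuzzles, while UpdateRespawn moves the respawn point.
; An unconnected fragment would refill submarine oxygen but never runs.
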(event `self.K2_PostLogin`
  (params (NewPlayer :type "PlayerController Object Reference"))
  (bind _returnvalue (`GameplayStatics.GetActorOfClass` "/Script/Engine.PlayerStart"))
  (set `self.RespawnLocation` (`self.GetTransform` _returnvalue))
  (bind _output_get (set `self.Controller Reference` NewPlayer))
  (`self.RestartPlayer` _output_get))

(event `self.K2_OnRestartPlayer`
  (params (NewPlayer :type "Controller Object Reference"))
  (add `self.OnDestroyed` (`Controller.K2_GetPawn` NewPlayer) (delegate `Respawn`)))

(event `Respawn` :!signature `self.OnDestroyed`
  (params (DestroyedActor :type "Actor Object Reference"))
  (bind (_respawnlocation_location _respawnlocation_rotation) (`KismetMathLibrary.BreakTransform` (`self.RespawnLocation`)))
  (set `self.FirstSpawn` false)
  (`self.RestartPlayerAtTransform` (`self.Controller Reference`) (`KismetMathLibrary.MakeTransform` _respawnlocation_location _respawnlocation_rotation))
  (`self.ResetPuzzles`))

(event `/Game/Checkpoint/BPI_UpdateRespawnLocation.UpdateRespawn`
  (params (NewSpawn :type "Transform Structure"))
  (set `self.RespawnLocation` (`KismetMathLibrary.MakeTransform` NewSpawn_Location NewSpawn_Rotation)))

(fn `UserConstructionScript`)