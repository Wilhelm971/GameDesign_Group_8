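; BP_LoreTablet is an interactable tablet that shows lore text to the player in a pop-up widget.
; On BeginPlay it looks up its text in the LoreTextStruct map, using its tablet ID enum converted to a name as the key.
; Interacting creates the widget, pauses the game and switches to UI-only input with a visible cursor.
; A close event bound to the widget removes it and restores gameplay input.
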(event `self.ReceiveBeginPlay`
  (set `self.LoreText` (`BlueprintMapLibrary.Map_Find` (`.LoreTextMap_5_8ED6A0434273B0787BC4BA8E87E5A4AD` (break `/Game/Martin/Blueprints/LoreTablet/F_LoreTextStruct` (`self.LoreTextStruct`))) (`KismetStringLibrary.Conv_StringToName` (`|GetEnumeratorNameAsString` (`self.LoreTabletID`))))))

(event `Interact_Interface.OnInteract`
  (params (CausingActor :type "Actor Object Reference"))
  (bind _returnvalue (`GameplayStatics.GetPlayerController` 0))
  (bind _returnvalue_2 (`|CreateWidget` "/Game/UI/WBP_LoreTabletWidget.WBP_LoreTabletWidget_C"))
  (`UserWidget.AddToViewport` _returnvalue_2 0)
  (`/Game/UI/WBP_LoreTabletWidget.SetLoreText` _returnvalue_2 (`self.LoreText`))
  (`GameplayStatics.SetGamePaused` true)
  (set `PlayerController.bShowMouseCursor` true _returnvalue)
  (`WidgetBlueprintLibrary.SetInputMode_UIOnlyEx` _returnvalue _returnvalue_2)
  (add `/Game/UI/WBP_LoreTabletWidget.CloseLoreTablet` _returnvalue_2 (delegate `CloseLoreTablet_Event`)))

(event `CloseLoreTablet_Event`
  (bind _returnvalue (`GameplayStatics.GetPlayerController` 0))
  (`Widget.RemoveFromParent` (stale `Interact_Interface.OnInteract` _returnvalue_2))
  (`GameplayStatics.SetGamePaused` false)
  (set `PlayerController.bShowMouseCursor` false _returnvalue)
  (`WidgetBlueprintLibrary.SetInputMode_GameOnly` _returnvalue))

(fn `UserConstructionScript`)