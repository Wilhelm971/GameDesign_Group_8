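; Oxygen bubble pickup on animated seaweed that refills the submarine player's oxygen on overlap, then respawns after a delay.
; A spawn timeline raises and scales the bubble as the kelp wraps, re-enabling the hit box and resetting the pickup gate.
; Overlap triggers the unwrap animation, a trigger parameter and Niagara splat, while a second timeline bounces and shrinks the bubble toward the player before hiding it and restarting the cycle.
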(event `Bubble Spawn`
  (bind _oxygen (`self.Oxygen`))
  (bind _oxygen_2 (`self.Oxygen`))
  (bind _bubble_seaweed (`self.Bubble_Seaweed`))
  (bind _oxygen_3 (`self.Oxygen`))
  (bind _oxygen_4 (`self.Oxygen`))
  (bind _returnvalue (`SceneComponent.K2_GetComponentLocation` _oxygen))
  (bind _returnvalue_2 (`SceneComponent.K2_GetComponentLocation` (`self.DefaultSceneRoot`)))
  (`PrimitiveComponent.SetCollisionResponseToAllChannels` (`self.HitBox`) "ECR_Overlap")
  (`SkeletalMeshComponent.PlayAnimation` (`self.Bubble_Seaweed`) "/Game/Meshes/Foliage/OxygenBubblePlant/Bubble_Kelp_Small_flat_wrap_Anim_Wrap.Bubble_Kelp_Small_flat_wrap_Anim_Wrap" false)
  (`SceneComponent.SetVisibility` (`self.Oxygen`) true false)
  (bind (_direction _bubble_spawn) (`Timeline|SpawnBubbel` :!via `PlayFromStart`)
    (:`Update`
      (`SceneComponent.K2_SetWorldLocation` _oxygen_4 (`KismetMathLibrary.VLerp` (+ _returnvalue_2 (0.0 0.0 -200.0)) (+ _returnvalue_2 (0.0 0.0 40.0)) _bubble_spawn) false false)
      (`SceneComponent.SetWorldScale3D` _oxygen_4 (`KismetMathLibrary.VLerp` (0.0 0.0 0.0) (0.7 0.7 0.7) _bubble_spawn))
      (set `self.bIsPopped` false)
      (goto _label :!via `Reset`))))

(event `BubblePop`
  (`SkeletalMeshComponent.PlayAnimation` (`self.Bubble_Seaweed`) "/Game/Meshes/Foliage/OxygenBubblePlant/Bubble_Kelp_Small_flat_wrap_Anim_Unwrap.Bubble_Kelp_Small_flat_wrap_Anim_Unwrap" false)
  (`PrimitiveComponent.SetCollisionResponseToAllChannels` (`self.HitBox`) "ECR_Ignore")
  (`AudioParameterControllerInterface.SetTriggerParameter` (`self.Bubble`) "Bubble Pick up"))

(event `self.ReceiveBeginPlay`
  (`self.Bubble Spawn`))

(event `self.HitBox.OnComponentBeginOverlap`
  (params (OverlappedComponent :type "PrimitiveComponent Object Reference") (OtherActor :type "Actor Object Reference") (OtherComp :type "PrimitiveComponent Object Reference") (OtherBodyIndex :type Integer) (bFromSweep :type Boolean) (SweepResult :type "HitResult Structure (by ref)"))
  (bind _returnvalue (`self.K2_GetActorLocation` OtherActor))
  (bind _oxygen (`self.Oxygen`))
  (bind _oxygen_2 (`self.Oxygen`))
  (bind _bubble_seaweed (`self.Bubble_Seaweed`))
  (bind _oxygen_3 (`self.Oxygen`))
  (bind _returnvalue_2 (`SceneComponent.K2_GetComponentLocation` _oxygen))
  (bind _z (.z (+ _returnvalue (* (`self.GetActorForwardVector` OtherActor) -80.0) (0.0 0.0 50.0))))
  (if (not (`self.bIsPopped`))
    (bind _asbp_submarine_player (cast `/Game/Wilhelm/Blueprints/BP_SubmarinePlayer` OtherActor))
    (`/Game/Wilhelm/Blueprints/BP_SubmarinePlayer.SetNewOxygen` _asbp_submarine_player 100.0)
    (set `self.bIsPopped` true)
    (`/Engine/EditorBlueprintResources/StandardMacros.DoOnce` false :!label _label
      (:`Completed`
        (`self.BubblePop`)
        (if (== OtherActor (`GameplayStatics.GetPlayerPawn` 0))
          (`KismetSystemLibrary.PrintString` "Hello")
          (`NiagaraFunctionLibrary.SpawnSystemAtLocation` "/Game/VFX/BubbleSplat.BubbleSplat" (`SceneComponent.K2_GetComponentLocation` _oxygen_3))
          (bind (_direction _alpha _bounce_) (`Timeline|BubblePickUp` :!via `PlayFromStart`)
            (:`Update`
              (`SceneComponent.K2_SetWorldRotation` _oxygen_3 (`KismetMathLibrary.Conv_VectorToRotator` (`KismetMathLibrary.Normal` (- _returnvalue _returnvalue_2))) false false)
              (`SceneComponent.K2_SetWorldLocation` _oxygen_3 (`KismetMathLibrary.VLerp` _returnvalue_2 (`KismetMathLibrary.MakeVector` (.x (+ _returnvalue (* (`self.GetActorForwardVector` OtherActor) -80.0) (0.0 0.0 50.0))) (.y (+ _returnvalue (* (`self.GetActorForwardVector` OtherActor) -80.0) (0.0 0.0 50.0))) (`KismetMathLibrary.Lerp` _z (+ _z 20.0) _bounce_)) _alpha) false false)
              (`SceneComponent.SetWorldScale3D` _oxygen_3 (`KismetMathLibrary.VLerp` (`SceneComponent.K2_GetComponentScale` _oxygen) (0.0 0.0 0.0) (* _alpha 1.0))))
            (:`Finished`
              (`SceneComponent.SetVisibility` _oxygen_2 false false)
              (`SceneComponent.K2_SetWorldLocation` _oxygen_2 (`SceneComponent.K2_GetComponentLocation` _bubble_seaweed) false false)
              (`SceneComponent.K2_SetWorldRotation` _oxygen_2 (`SceneComponent.K2_GetComponentRotation` _bubble_seaweed) false false)
              (`KismetSystemLibrary.Delay` 10.0)
              (set `self.bIsPopped` true)
              (`self.Bubble Spawn`))))))))

(fn `UserConstructionScript`)