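; Test player submarine pawn driven by physics, with a draining oxygen supply that quits the game once below zero.
; Enhanced Input applies forces for thrust (half strength in reverse) and elevation, torque for turning, and controller input for looking.
; Tick prints remaining oxygen and interpolates pitch and roll toward level.
; Interact input and overlaps are forwarded to a C++ interaction component, while bubble effect nodes are left unwired.
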(event `self.ReceiveBeginPlay`
  ; Binding Input
  (set `self.OxygenMeter` 200.0)
  (`EnhancedInputSubsystemInterface.AddMappingContext` (pcsubsystem `EnhancedInputLocalPlayerSubsystem` (`GameplayStatics.GetPlayerController` 0)) "/Game/Martin/INPUT/IMC_InputMapping.IMC_InputMapping" 0 (struct)))

(event `EnhancedInput|/Game/Martin/INPUT/IA_Look`
  (params (ActionValue :type "Vector2D Structure") (ElapsedSeconds :type "Float (double-precision)") (TriggeredSeconds :type "Float (double-precision)") (InputAction :type "InputAction Object Reference" :default "/Game/Martin/INPUT/IA_Look.IA_Look"))
  (bind (_x _y) (`KismetMathLibrary.BreakVector2D` ActionValue))
  ; Looks around
  (:`Triggered`
    (`self.AddControllerYawInput` _x)
    (`self.AddControllerPitchInput` _y)))

(event `EnhancedInput|/Game/Martin/INPUT/IA_Move`
  (params (ActionValue :type "Vector2D Structure") (ElapsedSeconds :type "Float (double-precision)") (TriggeredSeconds :type "Float (double-precision)") (InputAction :type "InputAction Object Reference" :default "/Game/Martin/INPUT/IA_Move.IA_Move"))
  (bind (_x _y) (`KismetMathLibrary.BreakVector2D` ActionValue))
  (bind _moveforce (`self.MoveForce`))
  (bind _submarine (`self.Submarine`))
  (bind _returnvalue (`SceneComponent.GetForwardVector` _submarine))
  ; Moves using Physics
  (:`Triggered`
    (if (< _y 0.0)
      (`PrimitiveComponent.AddForce` _submarine (* _y _moveforce 0.5 _returnvalue) "None" false)
      (else
        (`PrimitiveComponent.AddForce` _submarine (* _y _moveforce _returnvalue) "None" false)))))

(event `EnhancedInput|/Game/Martin/INPUT/IA_Rotate`
  (params (ActionValue :type "Float (double-precision)") (ElapsedSeconds :type "Float (double-precision)") (TriggeredSeconds :type "Float (double-precision)") (InputAction :type "InputAction Object Reference" :default "/Game/Martin/INPUT/IA_Rotate.IA_Rotate"))
  (bind _submarine (`self.Submarine`))
  ; Rotates Using Physics
  (:`Triggered`
    (`PrimitiveComponent.AddTorqueInRadians` _submarine (* ActionValue (`self.TorqueForce`) (`SceneComponent.GetUpVector` _submarine)) "None" false)))

(event `EnhancedInput|/Game/Martin/INPUT/IA_Elevate`
  (params (ActionValue :type "Vector2D Structure") (ElapsedSeconds :type "Float (double-precision)") (TriggeredSeconds :type "Float (double-precision)") (InputAction :type "InputAction Object Reference" :default "/Game/Martin/INPUT/IA_Elevate.IA_Elevate"))
  (bind _submarine (`self.Submarine`))
  ; Elevates Using Physics
  (:`Triggered`
    (`PrimitiveComponent.AddForce` _submarine (* (`.Y` (`KismetMathLibrary.BreakVector2D` ActionValue)) (`self.ElevateForce`) (`SceneComponent.GetUpVector` _submarine)) "None" false)))

(event `EnhancedInput|/Game/Martin/INPUT/IA_Interact`
  (params (ActionValue :type Boolean) (ElapsedSeconds :type "Float (double-precision)") (TriggeredSeconds :type "Float (double-precision)") (InputAction :type "InputAction Object Reference" :default "/Game/Martin/INPUT/IA_Interact.IA_Interact"))
  ; Binds Interact
  (:`Started`
    (`KismetSystemLibrary.PrintString` "Hello")
    (`CPP_CharacterInteractionComponent.OnInteract` (`self.CPP_CharacterInteraction`))))

(event `Interact_Interface.BeginOverlap`
  (params (CausingActor :type "Actor Object Reference"))
  ; Handles Interaction, THIS IS MEANT TO BE DONE IN C++
  (`CPP_CharacterInteractionComponent.OnBeginOverlap` (`self.CPP_CharacterInteraction`) CausingActor))

(event `Interact_Interface.EndOverlap`
  (params (CausingActor :type "Actor Object Reference"))
  ; Handles Interaction, THIS IS MEANT TO BE DONE IN C++
  (`CPP_CharacterInteractionComponent.OnEndOverlap` (`self.CPP_CharacterInteraction`) CausingActor))

(event `self.ReceiveTick`
  (params (DeltaSeconds :type "Float (single-precision)"))
  (bind _submarine (`self.Submarine`))
  (bind (_returnvalue_roll _returnvalue_pitch _returnvalue_yaw) (`KismetMathLibrary.BreakRotator` (`SceneComponent.K2_GetComponentRotation` _submarine)))
  (bind (_relativerotation_roll _relativerotation_pitch _relativerotation_yaw) (`KismetMathLibrary.BreakRotator` (`SceneComponent.RelativeRotation` _submarine)))
  (if (< (`self.OxygenMeter`) 0.0)
    (`KismetSystemLibrary.QuitGame` null "Quit")
    (else
      (`self.UseOxygen` DeltaSeconds)
      ; Straigtens boat to horizon
      (if (> (`KismetMathLibrary.Abs` _returnvalue_yaw) 0.0)
        (`self.K2_SetActorRotation` (`KismetMathLibrary.RInterpTo` (`KismetMathLibrary.MakeRotator` _returnvalue_roll _returnvalue_pitch _returnvalue_yaw) (`KismetMathLibrary.MakeRotator` _returnvalue_roll 0.0 _returnvalue_yaw) DeltaSeconds 1.0))
        (`self.K2_SetActorRelativeRotation` (`KismetMathLibrary.RInterpTo` (`KismetMathLibrary.MakeRotator` _relativerotation_roll _relativerotation_pitch _relativerotation_yaw) (`KismetMathLibrary.MakeRotator` 0.0 _relativerotation_pitch _relativerotation_yaw) DeltaSeconds 1.0))))))

(fn `UseOxygen`
  (params (DeltaTime :type "Float (double-precision)"))
  (bind _output_get (set `self.OxygenMeter` (- (`self.OxygenMeter`) DeltaTime)))
  (`KismetSystemLibrary.PrintString` (`KismetStringLibrary.Concat_StrStr` "OXYGEN: " (`KismetStringLibrary.Conv_DoubleToString` _output_get)) true false (struct :`G` 0.66 :`B` 1.0 :`A` 1.0) DeltaTime))

(fn `UserConstructionScript`)