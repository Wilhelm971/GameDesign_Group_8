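; BP_Geyser is an intermittent geyser that launches and lifts the player's physics submarine upward.
; A looping timer with random start variance flips the particle effect and capsule overlap response on and off, restarting itself with alternating short and long intervals.
; Entering the capsule applies an upward velocity impulse to the submarine, and Tick keeps adding upward acceleration until it exits.
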(event `self.ReceiveBeginPlay`
  (`KismetSystemLibrary.K2_SetTimerDelegate` (delegate `GeyserToggle`) (`self.GeyserTimer`) true false 0.0 2.0 :!label _label))

(event `ResetTimer`
  (`/Engine/EditorBlueprintResources/StandardMacros.FlipFlop`
    (:`A`
      (set `self.GeyserTimer` 3.0)
      (goto _label))
    (:`B`
      (set `self.GeyserTimer` 6.0)
      (goto _label))))

(event `GeyserToggle`
  (bind _geyserparticle (`self.GeyserParticle`))
  (bind _capsule (`self.Capsule`))
  (`/Engine/EditorBlueprintResources/StandardMacros.FlipFlop`
    (:`A`
      (`ActorComponent.Activate` _geyserparticle false)
      (`PrimitiveComponent.SetCollisionResponseToAllChannels` _capsule "ECR_Overlap")
      (`self.ResetTimer`))
    (:`B`
      (`ActorComponent.Deactivate` _geyserparticle)
      (`PrimitiveComponent.SetCollisionResponseToAllChannels` _capsule "ECR_Ignore")
      (`self.ResetTimer`))))

(event `self.ReceiveTick`
  (params (DeltaSeconds :type "Float (single-precision)"))
  (if (`self.bIsInGeyser`)
    (`PrimitiveComponent.AddForce` (`self.Player`) (0.0 0.0 400.0) "None" true)))

(event `self.Capsule.OnComponentBeginOverlap`
  (params (OverlappedComponent :type "PrimitiveComponent Object Reference") (OtherActor :type "Actor Object Reference") (OtherComp :type "PrimitiveComponent Object Reference") (OtherBodyIndex :type Integer) (bFromSweep :type Boolean) (SweepResult :type "HitResult Structure (by ref)"))
  (if (== OtherActor (`GameplayStatics.GetPlayerPawn` 0))
    (`KismetSystemLibrary.PrintString` "You are player")
    (bind _asbp_physics_submarine_test (cast `/Game/Martin/Blueprints/BP_PhysicsSubmarineTest` OtherActor))
    (bind _submarine (`/Game/Martin/Blueprints/BP_PhysicsSubmarineTest.Submarine` _asbp_physics_submarine_test))
    (set `self.Player` _submarine)
    (`PrimitiveComponent.AddImpulse` _submarine (0.0 0.0 100.0) "None" true)
    (set `self.bIsInGeyser` true)))

(event `self.Capsule.OnComponentEndOverlap`
  (params (OverlappedComponent :type "PrimitiveComponent Object Reference") (OtherActor :type "Actor Object Reference") (OtherComp :type "PrimitiveComponent Object Reference") (OtherBodyIndex :type Integer))
  (cast `/Game/Martin/Blueprints/BP_PhysicsSubmarineTest` OtherActor)
  (set `self.bIsInGeyser` false))

(fn `UserConstructionScript`)