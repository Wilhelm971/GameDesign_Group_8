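; AC_CreatureDamage is an actor component that lets a creature hurt the submarine player on contact.
; It binds to the begin overlap of the owner's capsule and, when a BP_SubmarinePlayer touches it, calls SetNewOxygen with the damage amount and notifies the owner through OnDamageMessage.
; A timer counted down in Tick enforces a five-second cooldown between hits.
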(event `self.ReceiveBeginPlay`
  (add `PrimitiveComponent.OnComponentBeginOverlap` (`Actor.GetComponentByClass` (`self.GetOwner`) "/Script/Engine.CapsuleComponent") (delegate `OnComponentBeginOverlap_Event`)))

(event `OnComponentBeginOverlap_Event`
  (params (OverlappedComponent :type "PrimitiveComponent Object Reference") (OtherActor :type "Actor Object Reference") (OtherComp :type "PrimitiveComponent Object Reference") (OtherBodyIndex :type Integer) (bFromSweep :type Boolean) (SweepResult :type "HitResult Structure (by ref)"))
  (if (< (`self.DamageTimer`) 0.0)
    (bind _asbp_submarine_player (cast `/Game/Wilhelm/Blueprints/BP_SubmarinePlayer` OtherActor))
    (`/Game/Wilhelm/Blueprints/BP_SubmarinePlayer.SetNewOxygen` _asbp_submarine_player (`self.DamageAmount`))
    (`KismetSystemLibrary.PrintString` "ELL BUZZED YOU")
    (message `/Game/Martin/Blueprints/BPI_CreatureInterface.OnDamage` (`self.GetOwner`))
    (set `self.DamageTimer` 5.0)))

(event `self.ReceiveTick`
  (params (DeltaSeconds :type "Float (single-precision)"))
  (set `self.DamageTimer` (- (`self.DamageTimer`) DeltaSeconds)))