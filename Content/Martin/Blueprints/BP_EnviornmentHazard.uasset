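; BP_EnviornmentHazard is an environmental hazard that penalizes the player submarine on contact.
; When its Box is overlapped by a BP_SubmarinePlayer, it passes DamageNumber to the submarine's SetNewOxygen.
; It then knocks the submarine back with a fixed-strength, mass-independent impulse on the player's Box, opposite to the root component's velocity.
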(event `self.Box.OnComponentBeginOverlap`
  (params (OverlappedComponent :type "PrimitiveComponent Object Reference") (OtherActor :type "Actor Object Reference") (OtherComp :type "PrimitiveComponent Object Reference") (OtherBodyIndex :type Integer) (bFromSweep :type Boolean) (SweepResult :type "HitResult Structure (by ref)"))
  (bind _asbp_submarine_player (cast `/Game/Wilhelm/Blueprints/BP_SubmarinePlayer` OtherActor))
  (if (== (`GameplayStatics.GetObjectClass` OverlappedComponent) "/Script/Engine.BoxComponent")
    (`/Game/Wilhelm/Blueprints/BP_SubmarinePlayer.SetNewOxygen` _asbp_submarine_player (`self.DamageNumber`))
    (`PrimitiveComponent.AddImpulse` (`PlayerSubmarine.Box` _asbp_submarine_player) (* (`KismetMathLibrary.Normal` (`SceneComponent.GetComponentVelocity` (`Actor.RootComponent` _asbp_submarine_player))) -500.0) "None" true)))

(fn `UserConstructionScript`)