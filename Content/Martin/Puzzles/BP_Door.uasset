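; Puzzle door actor that slides its door component upward when its OnEvent is triggered.
; OnEvent prints a debug message, starts the Open audio and plays the OpeningAnimation timeline from the start.
; Each timeline update lerps the door's world position from the scene root to a point above it, and also calls a fade-out on the audio.
; The Blueprint has no closing logic.
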(event `/Game/Martin/Puzzles/BPI_EventInterface.OnEvent`
  (bind _returnvalue (`SceneComponent.K2_GetComponentLocation` (`self.DefaultSceneRoot`)))
  (`KismetSystemLibrary.PrintString` "OPENING DOOR")
  (`AudioComponent.Play` (`self.Open`) 0.0)
  (bind (_direction _open) (`Timeline|OpeningAnimation` :!via `PlayFromStart`)
    (:`Update`
      (`SceneComponent.K2_SetWorldLocation` (`self.Door`) (`KismetMathLibrary.VLerp` _returnvalue (+ _returnvalue (0.0 0.0 200.0)) _open) false false)
      (`AudioComponent.FadeOut` (`self.Open`) 0.5 0.0 "Linear"))))

(fn `UserConstructionScript`)