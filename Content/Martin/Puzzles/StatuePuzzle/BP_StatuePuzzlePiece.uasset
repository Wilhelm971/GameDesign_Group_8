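; BP_StatuePuzzlePiece is an interactable piece of the statue puzzle with a configurable starting orientation.
; The construction script maps the initial rotation setting to quarter-turn yaw steps on the static mesh.
; It caches the mesh's world rotation at BeginPlay, and a ResetRotation event restores it.
; Interaction calls the parent handler, then plays rotation audio that fades out after a short delay.
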(event `self.ReceiveBeginPlay`
  (set `self.Start Rotation` (`SceneComponent.K2_GetComponentRotation` (`self.StaticMesh`))))

(event `ResetRotation`
  (`SceneComponent.K2_SetWorldRotation` (`self.StaticMesh`) (`self.Start Rotation`) false false))

(event `Interact_Interface.OnInteract`
  (params (CausingActor :type "Actor Object Reference"))
  (bind _rotateaudio (`self.RotateAudio`))
  (`parent.OnInteract` CausingActor)
  (`AudioComponent.Play` _rotateaudio 0.0)
  (`KismetSystemLibrary.Delay` 2.0)
  (`AudioComponent.FadeOut` _rotateaudio 1.0 0.0 "Linear"))

(fn `UserConstructionScript`
  (bind _staticmesh (`self.StaticMesh`))
  (switch `int` (`self.InititialRotation`)
    (:`Default`
      (`SceneComponent.K2_SetRelativeRotation` :`self` _staticmesh :!label _label))
    (:`0`
      (goto _label))
    (:`1`
      (`SceneComponent.K2_SetRelativeRotation` _staticmesh (struct :`Yaw` 90.0) false false))
    (:`2`
      (`SceneComponent.K2_SetRelativeRotation` _staticmesh (struct :`Yaw` 180.0) false false))
    (:`3`
      (`SceneComponent.K2_SetRelativeRotation` _staticmesh (struct :`Yaw` 270.0) false false))))