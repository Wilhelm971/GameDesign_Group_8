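; BP_StatuePuzzleManager handles resetting the statue puzzle while it is unsolved.
; On BeginPlay it binds ResetPuzzle to the puzzle reset event of BP_GameModeForTesting.
; A reset zeroes the rotation position of each BP_StatuePuzzlePiece in PuzzlePieces and calls its ResetRotation, unless PuzzleSolved is set.
; PuzzleSolved is only read here, and debug prints report whether the reset ran.
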(event `self.ReceiveBeginPlay`
  (bind _asbp_game_mode_for_testing (cast `/Game/Martin/Blueprints/BP_GameModeForTesting` (`GameplayStatics.GetGameMode`)))
  (add `/Game/Martin/Blueprints/BP_GameModeForTesting.ResetPuzzles` _asbp_game_mode_for_testing (delegate `ResetPuzzle`)))

(event `ResetPuzzle`
  (if (`self.bPuzzleSolved`)
    (`KismetSystemLibrary.PrintString` "Not Reset Puzzle")
    (else
      (`KismetSystemLibrary.PrintString` "Reset Puzzle")
      (for _array_element (`self.PuzzlePieces`)
        (bind _asbp_statue_puzzle_piece (cast `/Game/Martin/Puzzles/StatuePuzzle/BP_StatuePuzzlePiece` _array_element))
        (set `CPP_RotatingPuzzlePiece.RotationPosition` 0 _asbp_statue_puzzle_piece)
        (`/Game/Martin/Puzzles/StatuePuzzle/BP_StatuePuzzlePiece.ResetRotation` _asbp_statue_puzzle_piece)))))

(fn `UserConstructionScript`)