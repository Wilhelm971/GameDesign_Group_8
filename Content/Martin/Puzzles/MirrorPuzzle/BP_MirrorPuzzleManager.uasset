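; BP_MirrorPuzzleManager is a manager Blueprint that resets the pieces of a mirror puzzle.
; On BeginPlay it binds its ResetPuzzle event to the puzzle-reset event of BP_GameModeForTesting.
; When that fires and PuzzleSolved is true, it calls ResetPuzzle on each BP_MirrorPuzzlePiece in PuzzlePieces and zeroes its RotationPosition.
; The PuzzleSolved flag is only read here, never set or cleared.
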(event `self.ReceiveBeginPlay`
  (bind _asbp_game_mode_for_testing (cast `/Game/Martin/Blueprints/BP_GameModeForTesting` (`GameplayStatics.GetGameMode`)))
  (add `/Game/Martin/Blueprints/BP_GameModeForTesting.ResetPuzzles` _asbp_game_mode_for_testing (delegate `ResetPuzzle`)))

(event `ResetPuzzle`
  (if (`self.bPuzzleSolved`)
    (for _array_element (`self.PuzzlePieces`)
      (bind _asbp_mirror_puzzle_piece (cast `/Game/Martin/Puzzles/MirrorPuzzle/BP_MirrorPuzzlePiece` _array_element))
      (`/Game/Martin/Puzzles/MirrorPuzzle/BP_MirrorPuzzlePiece.ResetPuzzle` _asbp_mirror_puzzle_piece)
      (set `CPP_RotatingPuzzlePiece.RotationPosition` 0 _asbp_mirror_puzzle_piece))))

(fn `UserConstructionScript`)