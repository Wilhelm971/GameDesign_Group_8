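; BP_LoreTabletPuzzlePiece is an interactable piece of the lore tablet puzzle, showing an animal symbol decal and a light.
; Activation clears the highlight material and sets the light's "IsCorrect?" material parameter to 0, while resetting restores both.
; Both events print debug strings, then call the parent implementation.
; The construction script starts the light at 1 and applies the Decal material to the symbol.
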(event `self.OnActivated`
  (set `CPP_InteractableObjectComponent.HighlightMaterial` null (`self.InteractableObjectComponent`))
  (`KismetSystemLibrary.PrintString` "Balle")
  (`MeshComponent.SetScalarParameterValueOnMaterials` (`self.Light`) "IsCorrect?" 0.0)
  (`parent.OnActivated`))

(event `self.ResetPiece`
  (set `CPP_InteractableObjectComponent.HighlightMaterial` "/Game/Materials/MI_ObjectHighlight.MI_ObjectHighlight" (`self.InteractableObjectComponent`))
  (`KismetSystemLibrary.PrintString` "pung")
  (`MeshComponent.SetScalarParameterValueOnMaterials` (`self.Light`) "IsCorrect?" 1.0)
  (`parent.ResetPiece`))

(fn `UserConstructionScript`
  (`MeshComponent.SetScalarParameterValueOnMaterials` (`self.Light`) "IsCorrect?" 1.0)
  (`DecalComponent.SetDecalMaterial` (`self.AnimalSymbol`) (`self.Decal`)))