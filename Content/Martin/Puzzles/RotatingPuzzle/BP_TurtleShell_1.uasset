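; Turtle shell interactable for the rotating puzzle that plays a puzzle-solved sound on BeginPlay and a pickup sound on interact, after calling the parent's interact logic.
; Its Destroyed event acts as the trigger: it messages the Door, shakes the camera, spawns wall dust at a stored location and scale, and plays a shake sound.
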(event `self.ReceiveBeginPlay`
  (`GameplayStatics.PlaySound2D` "/Game/Audio/MetaSoundFiles/MSS_PuzzleSolved.MSS_PuzzleSolved" 1.0 1.0 0.0 null null))

(event `self.ReceiveDestroyed`
  (`KismetSystemLibrary.PrintString` "Tutel ødelagt")
  (message `/Game/Martin/Puzzles/BPI_EventInterface.OnEvent` (`self.Door`))
  (`LegacyCameraShake.StartLegacyCameraShake` (`PlayerController.PlayerCameraManager` (`GameplayStatics.GetPlayerController` 0)) "/Game/VFX/BP_CameraShake.BP_CameraShake_C")
  (`NiagaraFunctionLibrary.SpawnSystemAtLocation` "/Game/VFX/NS_WallDust.NS_WallDust" (`self.ParticleLocation`) (struct) (`self.ParticleSize`))
  (`GameplayStatics.PlaySound2D` "/Game/Audio/MetaSoundFiles/MSS_Shake.MSS_Shake" 1.0 1.0 0.0 null null))

(event `Interact_Interface.OnInteract`
  (params (CausingActor :type "Actor Object Reference"))
  (`parent.OnInteract` CausingActor)
  (`GameplayStatics.PlaySound2D` "/Game/Audio/MetaSoundFiles/MSS_PickUp.MSS_PickUp" 1.0 1.0 0.0 null null))

(fn `UserConstructionScript`)