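; Manager actor for a rotating pillar puzzle that resets its connected pieces, intended for when the player dies before solving it.
; On BeginPlay it binds its reset event to the testing game mode.
; Unless PuzzleSolved is set, a reset zeroes each tutorial puzzle piece's rotation position and calls its rotation reset.
; PuzzleSolved is only read here, and debug prints report whether the reset ran.
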(event `self.ReceiveBeginPlay`
  ; Resets Connected puzzlepieces if player dies before its solved
  (bind _asbp_game_mode_for_testing (cast `/Game/Martin/Blueprints/BP_GameModeForTesting` (`GameplayStatics.GetGameMode`)))
  (add `/Game/Martin/Blueprints/BP_GameModeForTesting.ResetPuzzles` _asbp_game_mode_for_testing (delegate `ResetPuzzle`)))

(event `ResetPuzzle`
  ; Resets Connected puzzlepieces if player dies before its solved
  (if (`self.bPuzzleSolved`)
    (`KismetSystemLibrary.PrintString` "Not Reset Puzzle")
    (else
      (`KismetSystemLibrary.PrintString` "Reset Puzzle")
      (for _array_element (`self.PuzzlePieces`)
        (bind _asbp_tutorial_puzzle_piece (cast `/Game/Martin/Puzzles/RotatingPuzzle/PuzzlePieces/BP_TutorialPuzzlePiece` _array_element))
        (set `CPP_RotatingPuzzlePiece.RotationPosition` 0 _asbp_tutorial_puzzle_piece)
        (`/Game/Martin/Puzzles/RotatingPuzzle/PuzzlePieces/BP_TutorialPuzzlePiece.ResetRotation` _asbp_tutorial_puzzle_piece)))))

(fn `UserConstructionScript`)