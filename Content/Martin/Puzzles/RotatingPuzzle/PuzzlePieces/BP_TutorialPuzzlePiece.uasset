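; BP_TutorialPuzzlePiece is a piece of the tutorial rotating puzzle that shows on a light orb whether it is correctly positioned.
; Each Tick compares RotationPosition to CorrectPosition and sets the orb's "IsCorrect?" material parameter, which is 0 when correct and 1 otherwise.
; BeginPlay stores the starting rotation, which ResetRotation restores on player death without changing RotationPosition.
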(event `self.ReceiveBeginPlay`
  (`MeshComponent.SetScalarParameterValueOnMaterials` (`self.SM_Light_orb`) "IsCorrect?" 1.0)
  (set `self.StartRotation` (`SceneComponent.K2_GetComponentRotation` (`self.RootComponent`))))

(event `self.ReceiveTick`
  (params (DeltaSeconds :type "Float (single-precision)"))
  (bind _sm_light_orb (`self.SM_Light_orb`))
  (if (== (`self.RotationPosition`) (`self.CorrectPosition`))
    (`MeshComponent.SetScalarParameterValueOnMaterials` _sm_light_orb "IsCorrect?" 0.0)
    (else
      (`MeshComponent.SetScalarParameterValueOnMaterials` _sm_light_orb "IsCorrect?" 1.0))))

(event `ResetRotation`
  ; Reset physical rotation when player dies
  (`self.K2_SetActorRotation` (`self.StartRotation`)))

(fn `UserConstructionScript`)