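; BP_MazePuzzlePiece is an interactable maze puzzle piece with a light ball that shows whether it is activated.
; Activation clears the highlight material, sets the ball's "IsCorrect?" material parameter to zero, runs the parent logic and plays LightOn.
; Reset restores the highlight and sets the parameter to one, matching the construction script's initial state, then runs the parent reset.
; Both events print debug strings.
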(event `self.OnActivated`
  (set `CPP_InteractableObjectComponent.HighlightMaterial` null (`self.InteractableObjectComponent`))
  (`KismetSystemLibrary.PrintString` "Balle")
  (`MeshComponent.SetScalarParameterValueOnMaterials` (`self.LightBall`) "IsCorrect?" 0.0)
  (`parent.OnActivated`)
  (`AudioComponent.Play` (`self.LightOn`) 0.0))

(event `self.ResetPiece`
  (set `CPP_InteractableObjectComponent.HighlightMaterial` "/Game/Materials/MI_ObjectHighlight.MI_ObjectHighlight" (`self.InteractableObjectComponent`))
  (`KismetSystemLibrary.PrintString` "pung")
  (`MeshComponent.SetScalarParameterValueOnMaterials` (`self.LightBall`) "IsCorrect?" 1.0)
  (`parent.ResetPiece`))

(fn `UserConstructionScript`
  (`MeshComponent.SetScalarParameterValueOnMaterials` (`self.LightBall`) "IsCorrect?" 1.0))