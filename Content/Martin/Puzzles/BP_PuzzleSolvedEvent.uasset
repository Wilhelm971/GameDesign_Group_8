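; Puzzle reward actor that spawns a turtle shell fragment when its PuzzleSolved event is called.
; The event prints a debug message and spawns a TurtleShellFragment at the actor's root location.
; It passes the connected door, particle location and size, and shell mesh to the fragment, makes the fragment's static mesh visible, then destroys itself.
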(event `self.PuzzleSolved`
  (`KismetSystemLibrary.PrintString` "I AM SOLVED NOW SPAWN THE TURTLE")
  (bind _returnvalue (`|SpawnActorFromClass` (`self.TurtleShellFragment`) (`KismetMathLibrary.MakeTransform` (`SceneComponent.K2_GetComponentLocation` (`self.SceneRoot`))) "Undefined" "MultiplyWithRoot" null null))
  (set `/Game/Martin/Puzzles/RotatingPuzzle/BP_TurtleShell_1.Door` (`self.ConnectedDoor`) _returnvalue)
  (set `/Game/Martin/Puzzles/RotatingPuzzle/BP_TurtleShell_1.ParticleLocation` (`self.ParticleLocation`) _returnvalue)
  (set `/Game/Martin/Puzzles/RotatingPuzzle/BP_TurtleShell_1.ParticleSize` (`self.ParticleSize`) _returnvalue)
  (set `/Game/Martin/Puzzles/RotatingPuzzle/BP_TurtleShell_1.TurtleShellMesh` (`self.Turtle Shell Mesh`) _returnvalue)
  (`SceneComponent.SetVisibility` (`CPP_InteractableObjectBase.StaticMesh` _returnvalue) true false)
  (`self.K2_DestroyActor`))

(fn `UserConstructionScript`)