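; BP_Checkpoint is an interactable checkpoint actor that sets the player's respawn point.
; Its first OnInteract disables the collision sphere and passes the Arrow's world transform to the game mode through UpdateRespawnMessage.
; It also switches the GlowOrb's "IsCorrect?" material parameter from the construction-time off value to on, then deactivates the particles and destroys them after a short delay.
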(event `Interact_Interface.OnInteract`
  (params (CausingActor :type "Actor Object Reference"))
  (bind _particles (`self.Particles`))
  (`KismetSystemLibrary.PrintString` "Checkpoint Activated")
  (`/Engine/EditorBlueprintResources/StandardMacros.DoOnce` false
    (:`Completed`
      (`PrimitiveComponent.SetCollisionEnabled` (`self.CollisionSphere`) "NoCollision")
      (message `/Game/Checkpoint/BPI_UpdateRespawnLocation.UpdateRespawn` (`GameplayStatics.GetGameMode`) (`SceneComponent.K2_GetComponentToWorld` (`self.Arrow`)))
      (`MeshComponent.SetScalarParameterValueOnMaterials` (`self.GlowOrb`) "IsCorrect?" 1.0)
      (`ActorComponent.Deactivate` _particles)
      (`KismetSystemLibrary.Delay` 5.0)
      (`ActorComponent.K2_DestroyComponent` _particles))))

(fn `UserConstructionScript`
  (`MeshComponent.SetScalarParameterValueOnMaterials` (`self.GlowOrb`) "IsCorrect?" 0.0))