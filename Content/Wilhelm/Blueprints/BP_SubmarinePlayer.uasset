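; Player submarine pawn whose oxygen acts as its life, refilled on respawn and playing a death sound once depleted.
; Tick feeds the HUD oxygen bar and eases pitch and roll back level with RInterpTo.
; Sprint doubles move force and oxygen drain, while SetNewOxygen applies external gains and damage.
; Interact input and overlaps forward to a C++ interaction component, alongside debug print and death-key leftovers.
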(event `self.ReceiveBeginPlay`
  ; Reset Oxygen when respawning (only after first spawn)
  (bind _asbp_test_level_gamemode (cast `/Game/UI/BP_TestLevelGamemode` (`GameplayStatics.GetGameMode`)))
  (if (not (`/Game/UI/BP_TestLevelGamemode.FirstSpawn` _asbp_test_level_gamemode))
    (set `self.CurrentOxygen` (`self.MaxOxygen`))
    (goto _label :!via `Reset`)))

(event `self.LostGame`
  ; Respawns Player
  (`self.K2_DestroyActor`))

(event `EnhancedInput|/Game/Martin/INPUT/IA_Death`
  (params (ActionValue :type Boolean) (ElapsedSeconds :type "Float (double-precision)") (TriggeredSeconds :type "Float (double-precision)") (InputAction :type "InputAction Object Reference" :default "/Game/Martin/INPUT/IA_Death.IA_Death"))
  ; Just for testing
  (:`Triggered`
    (`self.K2_DestroyActor`)))

(event `EnhancedInput|/Game/Martin/INPUT/IA_Interact`
  (params (ActionValue :type Boolean) (ElapsedSeconds :type "Float (double-precision)") (TriggeredSeconds :type "Float (double-precision)") (InputAction :type "InputAction Object Reference" :default "/Game/Martin/INPUT/IA_Interact.IA_Interact"))
  ; Binds Interact
  (:`Started`
    (`|PlayMontage` (`self.SubmarineMesh`) "/Game/AnimationBlueprints/AM_Interact.AM_Interact"
      (:`then`
        (`KismetSystemLibrary.PrintString` "Hello")
        (`CPP_CharacterInteractionComponent.OnInteract` (`self.CPP_CharacterInteraction`))))))

(event `Interact_Interface.BeginOverlap`
  (params (CausingActor :type "Actor Object Reference"))
  ; Handles Interaction, THIS IS MEANT TO BE DONE IN C++
  (`CPP_CharacterInteractionComponent.OnBeginOverlap` (`self.CPP_CharacterInteraction`) CausingActor))

(event `Interact_Interface.EndOverlap`
  (params (CausingActor :type "Actor Object Reference"))
  ; Handles Interaction, THIS IS MEANT TO BE DONE IN C++
  (`CPP_CharacterInteractionComponent.OnEndOverlap` (`self.CPP_CharacterInteraction`) CausingActor))

(event `self.ReceiveTick`
  (params (DeltaSeconds :type "Float (single-precision)"))
  ; Tick
  (set `self.Delta Seconds` DeltaSeconds)
  (`self.OxygenHUD`)
  (`self.StraightenBoat`)
  ; Plays Death sound i character dies
  (if (< (`self.CurrentOxygen`) 0.0)
    (`/Engine/EditorBlueprintResources/StandardMacros.DoOnce` false :!label _label
      (:`Completed`
        (`GameplayStatics.PlaySound2D` "/Game/Audio/MetaSoundFiles/MSS_Death.MSS_Death" 1.0 1.0 0.0 null null)))))

(event `OxygenHUD`
  ; Oxygen HUD
  (bind _asbp_in_game_hud (cast `/Game/UI/BP_InGameHUD` (`PlayerController.GetHUD` (`GameplayStatics.GetPlayerController` 0))))
  (bind _asbp_game_hudwidget (cast `/Game/UI/BP_GameHUDWidget` (`InGameHUD.HUDWidgetRef` _asbp_in_game_hud)))
  (set `/Game/UI/BP_GameHUDWidget.OxygenPercent_0` (`KismetMathLibrary.FClamp` (/ (`self.CurrentOxygen`) (`self.MaxOxygen`))) _asbp_game_hudwidget))

(event `StraightenBoat`
  (bind _box (`self.Box`))
  (bind _delta_seconds (`self.Delta Seconds`))
  (bind (_returnvalue_roll _returnvalue_pitch _returnvalue_yaw) (`KismetMathLibrary.BreakRotator` (`SceneComponent.K2_GetComponentRotation` _box)))
  (bind (_relativerotation_roll _relativerotation_pitch _relativerotation_yaw) (`KismetMathLibrary.BreakRotator` (`SceneComponent.RelativeRotation` _box)))
  ; Straigtens boat to horizon
  (if (> (`KismetMathLibrary.Abs` _returnvalue_yaw) 0.0)
    (`self.K2_SetActorRotation` (`KismetMathLibrary.RInterpTo` (`KismetMathLibrary.MakeRotator` _returnvalue_roll _returnvalue_pitch _returnvalue_yaw) (`KismetMathLibrary.MakeRotator` _returnvalue_roll 0.0 _returnvalue_yaw) _delta_seconds 1.0))
    (`self.K2_SetActorRelativeRotation` (`KismetMathLibrary.RInterpTo` (`KismetMathLibrary.MakeRotator` _relativerotation_roll _relativerotation_pitch _relativerotation_yaw) (`KismetMathLibrary.MakeRotator` 0.0 _relativerotation_pitch _relativerotation_yaw) _delta_seconds 1.0))))

(event `EnhancedInput|/Game/Martin/INPUT/IA_Sprint`
  (params (ActionValue :type Boolean) (ElapsedSeconds :type "Float (double-precision)") (TriggeredSeconds :type "Float (double-precision)") (InputAction :type "InputAction Object Reference" :default "/Game/Martin/INPUT/IA_Sprint.IA_Sprint"))
  (bind _moveforce (`self.MoveForce`))
  (bind _oxygendrainrate (`self.OxygenDrainRate`))
  ; "Sprint" -costs extra oxygen
  (:`Started`
    (set `self.MoveForce` (* _moveforce 2.0))
    (set `self.OxygenDrainRate` (* _oxygendrainrate 2.0)))
  (:`Completed`
    (set `self.MoveForce` (* _moveforce 0.5))
    (set `self.OxygenDrainRate` (* _oxygendrainrate 0.5))))

(event `SetNewOxygen`
  (params (Oxygen :type "Float (double-precision)"))
  (bind _maxoxygen (`self.MaxOxygen`))
  (bind _returnvalue (+ Oxygen (`self.CurrentOxygen`)))
  ; Function for oxygenplant and damage enteties to set player oxygen
  (if (< Oxygen 0.0)
    (`AudioComponent.Play` (`self.DamageSound`) 0.0))
  (if (> _returnvalue _maxoxygen)
    (set `self.CurrentOxygen` _maxoxygen)
    (else
      (set `self.CurrentOxygen` _returnvalue))))

(fn `UserConstructionScript`)